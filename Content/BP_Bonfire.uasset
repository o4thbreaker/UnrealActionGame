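; Bonfire actor that acts as an interactable save point, lighting its flames when used.
; Interact sets the fire active, has the ArtGameModeBase write the save game, prints a confirmation and refreshes the flames.
; OnActorLoaded runs the same flame update, which activates the Niagara effect if the fire is active and never turns it off.
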(event `UpdateFlames`
  (if (`self.IsFireActive`)
    (`ActorComponent.Activate` (`self.Niagara`) false)))

(event `ArtGameplayInterface.Interact`
  (params (InstitgatorPawn :type "Pawn Object Reference"))
  (set `self.IsFireActive` true)
  (bind _asart_game_mode_base (cast `ArtGameModeBase` (`GameplayStatics.GetGameMode`)))
  (`ArtGameModeBase.WriteSaveGame` _asart_game_mode_base)
  (`KismetSystemLibrary.PrintString` "WORLD SAVED" true true (struct :`R` 1.0 :`G` 0.48409 :`B` 0.105608 :`A` 1.0))
  (`self.UpdateFlames`))

(event `ArtGameplayInterface.OnActorLoaded`
  (`self.UpdateFlames`))

(fn `UserConstructionScript`)